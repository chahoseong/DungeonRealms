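; Base Gameplay Ability for melee attacks that plays a montage and supports input-driven combos.
; Montage gameplay events open and close the combo window, which also closes when the ability ends.
; Pressing input inside the window commits the combo and ends the ability, using a local-only end without authority.
; A hit-event wait is stubbed with no tag or handling, and nothing here calls it.
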(event `self.K2_ActivateAbility`
  (`AbilityTask_PlayMontageAndWait.CreatePlayMontageAndWaitProxy` "None" (`self.Montage to Play`)
    (:`then`
      (`self.WaitComboWindowEvent`))
    (:`OnCompleted`
      (`self.K2_EndAbility` :!label _label))
    (:`OnBlendOut`
      (goto _label))
    (:`OnInterrupted`
      (goto _label))
    (:`OnCancelled`
      (goto _label))))

(event `self.K2_OnEndAbility`
  (params (bWasCancelled :type Boolean))
  (if (`self.IsComboWindowOpen`)
    (`self.CloseComboWindow`)))

(event `self.K2_InputPressed`
  (if (`self.IsComboWindowOpen`)
    (`self.CommitCombo`)
    (`self.K2_HasAuthority`
      (:`True`
        (`self.K2_EndAbility`))
      (:`False`
        (`self.K2_EndAbilityLocally`)))))

(event `WaitComboWindowEvent`
  (`|ExecutionSequence`
    (:`then_0`
      (`AbilityTask_WaitGameplayEvent.WaitGameplayEvent` (struct :`TagName` "GameplayEvent.Montage.ComboWindow.Open") null
        (:`EventReceived`
          (`self.OpenComboWindow`))))
    (:`then_1`
      (`AbilityTask_WaitGameplayEvent.WaitGameplayEvent` (struct :`TagName` "GameplayEvent.Montage.ComboWindow.Close") null
        (:`EventReceived`
          (`self.CloseComboWindow`))))))

(event `WaitHitEvent`
  (`AbilityTask_WaitGameplayEvent.WaitGameplayEvent` (struct) null))